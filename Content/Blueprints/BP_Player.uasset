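; Player Blueprint that creates and shows the player HUD and runs a timed resource-gain task, apparently a debug prototype.
; On BeginPlay it adds WPB_PlayerHUD to the viewport and plays the TL_Task timeline.
; Timeline updates pass through a one-second Delay, then print a countdown lerped from Timer toward zero.
; Each pass also adds Timer times ResrouceToAdd to ResourcePlaceholder and prints the total.
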(event `self.ReceiveBeginPlay`
  (bind _returnvalue (`|CreateWidget` "/Game/Blueprints/WPB_PlayerHUD.WPB_PlayerHUD_C" (`self.GetLocalViewingPlayerController`)))
  (`UserWidget.AddToViewport` _returnvalue 0)
  (bind (_direction _tasktimer) (`Timeline|TL_Task`)
    (:`Update`
      (`KismetSystemLibrary.Delay` 1.0)
      (`KismetSystemLibrary.PrintString` (`KismetStringLibrary.Conv_IntToString` (`KismetStringLibrary.Conv_StringToInt` (`KismetStringLibrary.Conv_DoubleToString` (`KismetMathLibrary.Lerp` (`self.Timer`) 0.0 _tasktimer)))))
      (bind _output_get (set `self.ResourcePlaceholder` (+ (* (`self.Timer`) (`self.ResrouceToAdd`)) (`self.ResourcePlaceholder`))))
      (`KismetSystemLibrary.PrintString` (`KismetStringLibrary.Conv_IntToString` _output_get)))))

(fn `UserConstructionScript`)