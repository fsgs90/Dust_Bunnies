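; Player Blueprint that sets up the HUD, a prototype task timer and dust bunny spawning.
; BeginPlay adds WPB_PlayerHUD and disables gravity on the mesh and capsule.
; It also plays TL_Task, whose updates pass through a one-second Delay to print a countdown and accumulate placeholder resources.
; SpawnDustBunny spawns BP_DustBunny at the capsule's location, then moves the player's root to the world origin.
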(event `self.ReceiveBeginPlay`
  (`|ExecutionSequence`
    (:`then_0`
      (bind _returnvalue (`|CreateWidget` "/Game/Blueprints/WPB_PlayerHUD.WPB_PlayerHUD_C" (`self.GetLocalViewingPlayerController`)))
      (`UserWidget.AddToViewport` _returnvalue 0)
      (bind (_direction _tasktimer) (`Timeline|TL_Task`)
        (:`Update`
          (`KismetSystemLibrary.Delay` 1.0)
          (`KismetSystemLibrary.PrintString` (`KismetStringLibrary.Conv_IntToString` (`KismetStringLibrary.Conv_StringToInt` (`KismetStringLibrary.Conv_DoubleToString` (`KismetMathLibrary.Lerp` (`self.Timer`) 0.0 _tasktimer)))))
          (bind _output_get (set `self.ResourcePlaceholder` (+ (* (`self.Timer`) (`self.ResrouceToAdd`)) (`self.ResourcePlaceholder`))))
          (`KismetSystemLibrary.PrintString` (`KismetStringLibrary.Conv_IntToString` _output_get)))))
    (:`then_1`
      (`SkeletalMeshComponent.SetEnableBodyGravity` (`self.Mesh`) false "None")
      (`PrimitiveComponent.SetEnableGravity` (`self.CapsuleComponent`) false))))

(event `Spawn DustBunny`
  (`|SpawnActorFromClass` "/Game/Blueprints/BP_DustBunny.BP_DustBunny_C" (`KismetMathLibrary.Conv_VectorToTransform` (+ (`SceneComponent.K2_GetComponentLocation` (`self.CapsuleComponent`)) (0.0 0.0 0.0))) "Undefined" "MultiplyWithRoot" null null)
  (`KismetSystemLibrary.PrintString` "DustBB")
  (`SceneComponent.K2_SetWorldLocation` (`self.RootComponent`) (0.0 0.0 0.0) false false))

(fn `UserConstructionScript`)